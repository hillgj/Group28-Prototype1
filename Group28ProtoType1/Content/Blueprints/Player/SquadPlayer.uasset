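; SquadPlayer is a player Blueprint that drives its LocationToWorld component from a stored PlayerPosition transform.
; BeginPlay seeds PlayerPosition with the LocationToWorld world transform of player pawn 0, cast to SquadPlayer.
; Tick reapplies that location and rotation every frame, and nothing here updates the value afterwards.
; An under-cursor visibility trace with a normal-based rotation is left unconnected.
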(event EventBeginPlay
  ;[1 1 1] Set starting point
  (Variables|Movement|SetPlayerPosition (Transformation|GetWorldTransform (Variables|SquadPlayer_C|GetLocationToWorld (.AsSquad%20Player (Utilities|Casting|CastToSquadPlayer (Game|Player|GetPlayerPawn 0)))))))

(event EventTick
  (params (DeltaSeconds :type Float%20%28single-precision%29))
  (bind _playerposition (Variables|Movement|GetPlayerPosition))
  ;[1 1 1] Set Player Position
  (Transformation|SetWorldLocationAndRotation (Variables|Default|GetLocationToWorld) (.location _playerposition) (.rotation _playerposition) false false))

(fn ConstructionScript)