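; Enemy spawner for horde spawning that starts when the player character enters its sphere trigger.
; A DoOnce gates the overlap, and ResetSpawn re-arms it.
; Each wave uses a Sequence with staggered delays to spawn three AI characters at the spawner's transform, raised by SpawnHeight.
; The last Sequence branch calls SpawnInit after a delay, which re-enters the Sequence and repeats waves with no stop condition.
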(event OnComponentBeginOverlap(Sphere)
  (params (OverlappedComponent :type Primitive%20Component%20Object%20Reference) (OtherActor :type Actor%20Object%20Reference) (OtherComp :type Primitive%20Component%20Object%20Reference) (OtherBodyIndex :type Integer) (bFromSweep :type Boolean) (SweepResult :type Hit%20Result%20Structure%20%28by%20ref%29))
  (if (== OtherActor (Game|GetPlayerCharacter 0))
    (Utilities|FlowControl|DoOnce false
      (:Completed
        (Utilities|FlowControl|Sequence
          (:then_0
            (CallFunction|Spawn))
          (:then_1
            (Utilities|FlowControl|Delay 0.6)
            (CallFunction|Spawn))
          (:then_2
            (Utilities|FlowControl|Delay 1.0)
            (CallFunction|Spawn))
          (:then_3
            (Utilities|FlowControl|Delay 5.0)
            (CallFunction|SpawnInit)))))))

(event Custom|ResetSpawn
  (Utilities|FlowControl|DoOnce false) ; enters at Reset
)

(event Custom|Spawn
  (bind _returnvalue (Transformation|GetActorTransform))
  (Game|SpawnActorfromClass "/Game/Blueprints/AIZombies/Characters/AICharacter.AICharacter_C" (Math|Transform|MakeTransform (Math|Vector|MakeVector (.x (.location _returnvalue)) (.y (.location _returnvalue)) (+ (Variables|Default|GetSpawnHeight) (.z (.location _returnvalue)))) (.rotation _returnvalue) (.scale _returnvalue)) "AdjustIfPossibleButAlwaysSpawn" 0 0))

(event Custom|SpawnInit
  (Utilities|FlowControl|Sequence
    (:then_0
      (CallFunction|Spawn))
    (:then_1
      (Utilities|FlowControl|Delay 0.6)
      (CallFunction|Spawn))
    (:then_2
      (Utilities|FlowControl|Delay 1.0)
      (CallFunction|Spawn))
    (:then_3
      (Utilities|FlowControl|Delay 5.0)
      (CallFunction|SpawnInit))))

(fn ConstructionScript)