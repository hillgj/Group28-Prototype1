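; Player character Blueprint for twin-stick control, with movement on the right stick and aiming and firing on the left.
; Right stick axes feed scaled input vectors to CharacterMovement.
; Left stick input past a deadzone turns the Cube at constant interpolation speed, then waits a FireRate Delay.
; A visibility line trace built from Arrow1 and WeaponRange then serves as the shot, with debug drawing and no hit handling.
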(event EventLeftStickX
  (params (Axis :type Float%20%28single-precision%29))
  (bind _arrow1 (Variables|Default|GetArrow1))
  (bind _returnvalue (Math|Vector|GetForwardVector _arrow1))
  ;[1 1 1] Rotation
  (if (> (Math|Vector|VectorLength (Math|Vector|MakeVector (stale EventLeftStickY Axis) Axis 0.0)) 0.5)
    (Variables|Default|SetRotation (Math|Conversions|RotationFromXVector (Math|Vector|MakeVector (stale EventLeftStickY Axis) Axis 0.0)))
    (Transformation|SetRelativeRotation (Variables|Default|GetCube) (Class|KismetMathLibrary|RInterptoConstant (Transformation|GetWorldRotation (Variables|Default|GetCube)) (Variables|Default|GetRotation) (Utilities|Time|GetWorldDeltaSeconds) (Variables|Default|GetRotspeed)) false false)
    (Utilities|FlowControl|Delay (Variables|Default|GetFireRate))
    ;[1 1 1] Shooting
    (Collision|LineTraceByChannel _returnvalue (* (+ _returnvalue (Transformation|GetWorldLocation _arrow1)) (Variables|Default|GetWeaponRange)) "TraceTypeQuery1" false 0 "ForDuration")))

(event EventLeftStickY
  (params (Axis :type Float%20%28single-precision%29))
  (bind _arrow1 (Variables|Default|GetArrow1))
  (bind _returnvalue (Math|Vector|GetForwardVector _arrow1))
  ;[1 1 1] Rotation
  (if (> (Math|Vector|VectorLength (Math|Vector|MakeVector Axis (stale EventLeftStickX Axis) 0.0)) 0.5)
    (Variables|Default|SetRotation (Math|Conversions|RotationFromXVector (Math|Vector|MakeVector Axis (stale EventLeftStickX Axis) 0.0)))
    (Transformation|SetRelativeRotation (Variables|Default|GetCube) (Class|KismetMathLibrary|RInterptoConstant (Transformation|GetWorldRotation (Variables|Default|GetCube)) (Variables|Default|GetRotation) (Utilities|Time|GetWorldDeltaSeconds) (Variables|Default|GetRotspeed)) false false)
    (Utilities|FlowControl|Delay (Variables|Default|GetFireRate))
    ;[1 1 1] Shooting
    (Collision|LineTraceByChannel _returnvalue (* (+ _returnvalue (Transformation|GetWorldLocation _arrow1)) (Variables|Default|GetWeaponRange)) "TraceTypeQuery1" false 0 "ForDuration")))

(event EventRightStickX
  (params (Axis :type Float%20%28single-precision%29))
  ;[1 1 1] Movement
  (Class|PawnMovementComponent|AddInputVector (Variables|Character|GetCharacterMovement) (Math|Vector|MakeVector (* Axis (Variables|Default|GetCharacterSpeed)) (* (stale EventRightStickY Axis) (Variables|Default|GetCharacterSpeed)) 0.0) false))

(event EventRightStickY
  (params (Axis :type Float%20%28single-precision%29))
  ;[1 1 1] Movement
  (Class|PawnMovementComponent|AddInputVector (Variables|Character|GetCharacterMovement) (Math|Vector|MakeVector (* (stale EventRightStickX Axis) (Variables|Default|GetCharacterSpeed)) (* Axis (Variables|Default|GetCharacterSpeed)) 0.0) false))

(fn ConstructionScript)